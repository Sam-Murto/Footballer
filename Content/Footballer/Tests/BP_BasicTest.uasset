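; BP_BasicTest is a functional test that checks whether kicking a Football launches it upward.
; Preparation finishes the test as invalid when the Football reference is missing.
; On start it calls Kicked on the Football, then checks velocity every tick and succeeds once vertical speed reaches MinZSpeed.
; The graph has no explicit failure branch for a kick that stays below that speed.
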(event `self.ReceivePrepareTest`
  (if (not (`KismetSystemLibrary.IsValid` (`self.Football`)))
    (`self.FinishTest` "Invalid" "Missing Football")))

(event `self.ReceiveStartTest`
  (`/Game/Footballer/Blueprints/BP_Football.Kicked` (`self.Football`)))

(event `self.ReceiveTick`
  (params (DeltaSeconds :type "Float (single-precision)"))
  (bind (_returnvalue_x _returnvalue_y _returnvalue_z) (`KismetMathLibrary.BreakVector` (`self.GetVelocity` (`self.Football`))))
  (if (>= _returnvalue_z (`self.MinZSpeed`))
    (`self.FinishTest` "Succeeded")))

(fn `UserConstructionScript`)