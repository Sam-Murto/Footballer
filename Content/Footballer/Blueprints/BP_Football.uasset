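; Football actor that a footballer kicks into the air and switches between left and right X positions.
; Kicked, rate-limited by an interval, derives vertical launch speed from air time via kinematics, snaps X/Y and plays power-scaled hit effects.
; SwitchSides starts a crossing, which Tick drives with constant X velocity lasting that air time.
; Also handles foot-socket placement, fire streak effects and CVar-gated apex debug drawing.
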(event `self.ReceiveBeginPlay`)

(event `self.ReceiveTick`
  (params (DeltaSeconds :type "Float (single-precision)"))
  (set `self.TimeSinceKicked` (+ DeltaSeconds (`self.TimeSinceKicked`)))
  (`self.UpdateBallState` DeltaSeconds))

(fn `AttachToFootballer`
  (params (Footballer :type "/Game/Footballer/Characters/BPC_Footballer Object Reference"))
  (bind (_returnvalue_x _returnvalue_y) (`KismetMathLibrary.BreakVector` (`self.K2_GetActorLocation`)))
  (`self.K2_SetActorLocation` (`SceneComponent.GetSocketLocation` (`Character.Mesh` Footballer) "R_Foot") false true)
  (`PrimitiveComponent.IgnoreActorWhenMoving` (`self.StaticMeshComponent`) Footballer true)
  (set `self.Y` _returnvalue_y))

(fn `CalculateSwitchTime`
  (params (VerticalSpeed :type "Float (double-precision)"))
  (returns (SwitchTime :type "Float (double-precision)"))
  ;[1 1 1] Duration of switch should be twice the time to the jump apex
  (return (* (/ (* VerticalSpeed -1.0) (`MovementComponent.GetGravityZ` (`self.ProjectileMovement`))) 2.0)))

(fn `CalculateVerticalBallSpeed`
  (params (AirTime :type "Float (double-precision)"))
  (returns (VerticalSpeed :type "Float (double-precision)"))
  (return (* (* AirTime -0.5) (`MovementComponent.GetGravityZ` (`self.ProjectileMovement`)))))

(fn `DrawDebug`
  (params (Location :type "Vector Structure"))
  (bind _returnvalue (`KismetSystemLibrary.GetConsoleVariableBoolValue` "footballer.DebugDraw"))
  (if _returnvalue
    (`KismetSystemLibrary.DrawDebugSphere` Location 10.0 12 (struct :`R` 1.0 :`G` 0.077434 :`B` 0.177118 :`A` 1.0) 1.0)))

(fn `EnableSim`
  (set `ProjectileMovementComponent.bSimulationEnabled` true (`self.ProjectileMovement`)))

(fn `GetDestinationPoint`
  (params (Speed :type "Float (double-precision)"))
  (returns (Destination :type "Vector Structure"))
  (bind (_returnvalue_x _returnvalue_y _returnvalue_z) (`KismetMathLibrary.BreakVector` (`self.K2_GetActorLocation`)))
  (return (`KismetMathLibrary.MakeVector` _returnvalue_x _returnvalue_y (+ (.z (`.BoxExtent` (`self.GetActorBounds` true))) (+ _returnvalue_z (* (/ (* Speed Speed) (* (`MovementComponent.GetGravityZ` (`self.ProjectileMovement`)) 2.0)) -1.0))))))

(fn `GetXPosition`
  (returns (X :type "Float (double-precision)"))
  (bind _rightx (`self.RightX`))
  (bind _leftx (`self.LeftX`))
  (return (select `/Game/Footballer/Misc/EBallMovementType` (`self.BallState`) :`NewEnumerator0` _rightx :`NewEnumerator1` _leftx :`NewEnumerator2` _leftx :`NewEnumerator3` _rightx)))

(fn `Kicked`
  (params (Time :type "Float (double-precision)") (PowerRatio :type "Float (double-precision)"))
  (returns (`Successful Kick` :type Boolean))
  (bind _verticalspeed (`self.CalculateVerticalBallSpeed` Time))
  (bind (_returnvalue_x _returnvalue_y _returnvalue_z) (`KismetMathLibrary.BreakVector` (`self.K2_GetActorLocation`)))
  (bind _projectilemovement (`self.ProjectileMovement`))
  (bind _hitaudio (`self.HitAudio`))
  (bind (_velocity_x _velocity_y) (`KismetMathLibrary.BreakVector` (`MovementComponent.Velocity` _projectilemovement)))
  ;[1 1 1] using kinematic equations, determine peak height  and how much time it takes to reach
  (if (> (`self.TimeSinceKicked`) (`self.KickTimeInterval`))
    (`ProjectileMovementComponent.SetVelocityInLocalSpace` _projectilemovement (`KismetMathLibrary.MakeVector` _velocity_x _velocity_y _verticalspeed))
    (`self.K2_SetActorLocation` (`KismetMathLibrary.MakeVector` (`self.GetXPosition`) (`self.Y`) _returnvalue_z))
    (`ActorComponent.Activate` (`self.HitEffectSystem`) true)
    (`self.DrawDebug` (`self.GetDestinationPoint` _verticalspeed))
    (set `self.TimeSinceKicked` 0.0)
    (`AudioComponent.SetPitchMultiplier` _hitaudio PowerRatio)
    (`AudioComponent.SetVolumeMultiplier` _hitaudio (+ PowerRatio 0.2))
    (set `self.SwitchTime` Time)
    (`AudioComponent.Play` (`self.HitAudio`) 0.05)
    (return true)
    (else
      (return false))))

(fn `SetFireActive`
  (params (Active :type Boolean))
  (bind _streakeffectsystem (`self.StreakEffectSystem`))
  (bind _fireaudio (`self.FireAudio`))
  (if Active
    (`ActorComponent.Activate` _streakeffectsystem false)
    (if (not (`AudioComponent.IsPlaying` _fireaudio))
      (`AudioComponent.Play` _fireaudio 0.0))
    (else
      (`ActorComponent.Deactivate` _streakeffectsystem)
      (`AudioComponent.Stop` _fireaudio))))

(fn `SetHitSoundPitchMultiplier`
  (params (float :type "Float (double-precision)"))
  (`AudioComponent.SetPitchMultiplier` (`self.HitAudio`) float))

(fn `SetParticleColor`
  (params (Color :type "LinearColor Structure"))
  (`NiagaraComponent.SetVariableLinearColor` (`self.HitEffectSystem`) "ParticleColor" Color))

(fn `SetXPositions`
  (params (Left :type "Float (double-precision)") (Right :type "Float (double-precision)"))
  (set `self.LeftX` Left)
  (set `self.RightX` Right))

(fn `SwitchSides`
  (set `self.BallState` (select `/Game/Footballer/Misc/EBallMovementType` (`self.BallState`) :`NewEnumerator0` "NewEnumerator2" :`NewEnumerator1` "NewEnumerator3" :`NewEnumerator2` "NewEnumerator2" :`NewEnumerator3` "NewEnumerator3" :!type "/Game/Footballer/Misc/EBallMovementType Enum")))

(fn `UpdateBallState`
  (params (DeltaSeconds :type "Float (double-precision)"))
  (locals (DeltaTime :type "Float (double-precision)") (NewLocalVar :type "Vector Structure" :default (0.0 0.0 0.0)))
  (bind _projectilemovement (`self.ProjectileMovement`))
  (bind (_velocity_x _velocity_y _velocity_z) (`KismetMathLibrary.BreakVector` (`MovementComponent.Velocity` (`self.ProjectileMovement`))))
  (bind (_velocity_x_2 _velocity_y_2 _velocity_z_2) (`KismetMathLibrary.BreakVector` (`MovementComponent.Velocity` _projectilemovement)))
  (bind _returnvalue (+ (`self.BallInterpolation`) (/ (`local.DeltaTime`) (`self.SwitchTime`))))
  (bind _returnvalue_2 (/ (- (`self.RightX`) (`self.LeftX`)) (`self.SwitchTime`)))
  (bind _returnvalue_3 (>= _returnvalue 1.0))
  (bind _returnvalue_4 (`KismetMathLibrary.SelectFloat` _returnvalue 1.0 (< _returnvalue 1.0)))
  (set `local.DeltaTime` DeltaSeconds)
  (switch `/Game/Footballer/Misc/EBallMovementType` (`self.BallState`)
    (:`NewEnumerator2`
      (`ProjectileMovementComponent.SetVelocityInLocalSpace` (`self.ProjectileMovement`) (`KismetMathLibrary.MakeVector` (* _returnvalue_2 -1.0) _velocity_y _velocity_z))
      (set `self.BallInterpolation` _returnvalue_4)
      (if _returnvalue_3
        (set `self.BallInterpolation` 0.0)
        (set `self.BallState` "NewEnumerator1")
        (`ProjectileMovementComponent.SetVelocityInLocalSpace` _projectilemovement (`KismetMathLibrary.MakeVector` 0.0 _velocity_y_2 _velocity_z_2))))
    (:`NewEnumerator3`
      (`ProjectileMovementComponent.SetVelocityInLocalSpace` (`self.ProjectileMovement`) (`KismetMathLibrary.MakeVector` _returnvalue_2 _velocity_y _velocity_z))
      (set `self.BallInterpolation` _returnvalue_4)
      (if _returnvalue_3
        (set `self.BallInterpolation` 0.0)
        (set `self.BallState` "NewEnumerator0")
        (`ProjectileMovementComponent.SetVelocityInLocalSpace` _projectilemovement (`KismetMathLibrary.MakeVector` 0.0 _velocity_y_2 _velocity_z_2))))))

(fn `UserConstructionScript`)