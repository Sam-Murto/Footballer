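; Player footballer character for a ball-juggling game where left and right kicks keep a football airborne to build streaks.
; Kick inputs set a flick state, and Tick tests foot socket height and proximity to detect contact with the ball.
; A curve over kick timing sets air time and power, with downward contacts giving minimum power.
; Successful kicks advance streak stages, drive fire and color effects and randomly switch sides, while ball hits reset the streak.
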(event `self.ReceiveBeginPlay`
  (bind _mesh (`self.Mesh`))
  (bind _returnvalue_x (`KismetMathLibrary.BreakVector` (`SceneComponent.GetSocketLocation` _mesh "L_Foot")))
  (bind _returnvalue_x_2 (`KismetMathLibrary.BreakVector` (`SceneComponent.GetSocketLocation` _mesh "R_Foot")))
  (`self.InitGame`)
  (bind _returnvalue (`|CreateWidget` "/Game/Footballer/UI/W_Score.W_Score_C"))
  (bind _output_get (set `self.Widget` _returnvalue))
  (`UserWidget.AddToViewport` _output_get 0)
  (add `self.OnActorHit` (`self.Football`) (delegate `BallDropped`))
  (`/Game/Footballer/Blueprints/BP_Football.SetXPositions` (`self.Football`) _returnvalue_x _returnvalue_x_2)
  (bind _asbp_gamemode (cast `/Game/Footballer/Gamemode/BP_Gamemode` (`GameplayStatics.GetGameMode`)))
  (set `self.GameMode` _asbp_gamemode)
  (bind _asabp_footballer (cast `/Game/Footballer/Characters/ABP_Footballer` (`SkeletalMeshComponent.GetAnimInstance` (`self.Mesh`))))
  (bind _output_get_2 (set `/Game/Footballer/Characters/ABP_Footballer.AnimationSpeedMultiplier` (`self.AnimationSpeed`) _asabp_footballer))
  (set `self.TotalKickTime` (/ 0.8 _output_get_2)))

(event `BallDropped` :!signature `self.OnActorHit`
  (params (SelfActor :type "Actor Object Reference") (OtherActor :type "Actor Object Reference") (NormalImpulse :type "Vector Structure") (Hit :type "HitResult Structure (by ref)"))
  (`self.LoseStreak`))

(event `self.ReceiveTick`
  (params (DeltaSeconds :type "Float (single-precision)"))
  (if (`KismetSystemLibrary.IsValid` (`self.Football`))
    (switch `/Game/Footballer/Misc/EKickType` (`self.KickType`)
      (:`NewEnumerator0`
        (`self.UpdateFlick` "NewEnumerator0"))
      (:`NewEnumerator1`
        (`self.UpdateFlick` "NewEnumerator1")))))

(event `EnhancedInput|/Game/Footballer/InputActions/IA_RightKick`
  (params (ActionValue :type Boolean) (ElapsedSeconds :type "Float (double-precision)") (TriggeredSeconds :type "Float (double-precision)") (InputAction :type "InputAction Object Reference" :default "/Game/Footballer/InputActions/IA_RightKick.IA_RightKick"))
  (bind (_returnvalue_x _returnvalue_y _returnvalue_z) (`KismetMathLibrary.BreakVector` (`SceneComponent.GetSocketLocation` (`self.Mesh`) "R_Foot")))
  (:`Triggered`
    (switch `/Game/Footballer/Misc/EKickType` (`self.KickType`)
      (:`NewEnumerator2`
        (set `self.KickType` "NewEnumerator1")
        (set `self.kickStartTime` (`GameplayStatics.GetTimeSeconds`))
        (set `self.kickStartZ` _returnvalue_z))
      (:`NewEnumerator3`
        (`self.InitBall`)
        (`KismetSystemLibrary.Delay` 0.1)
        (`/Game/Footballer/Blueprints/BP_Football.Kicked` (`self.Football`) (`/Game/Footballer/Gamemode/BP_Gamemode.MaxBallAirTime` (`self.GameMode`)) 1.0)
        (set `self.KickType` "NewEnumerator2"))))
  (:`Canceled`
    (switch `/Game/Footballer/Misc/EKickType` (`self.KickType`) :!label _label
      (:`NewEnumerator0`
        _)
      (:`NewEnumerator1`
        _)
      (:`NewEnumerator2`
        _))
    (`self.ResetKick`))
  (:`Completed`
    (goto _label)))

(event `EnhancedInput|/Game/Footballer/InputActions/IA_LeftKick`
  (params (ActionValue :type Boolean) (ElapsedSeconds :type "Float (double-precision)") (TriggeredSeconds :type "Float (double-precision)") (InputAction :type "InputAction Object Reference" :default "/Game/Footballer/InputActions/IA_LeftKick.IA_LeftKick"))
  (bind (_returnvalue_x _returnvalue_y _returnvalue_z) (`KismetMathLibrary.BreakVector` (`SceneComponent.GetSocketLocation` (`self.Mesh`) "L_Foot")))
  (:`Triggered`
    (switch `/Game/Footballer/Misc/EKickType` (`self.KickType`)
      (:`NewEnumerator2`
        (set `self.KickType` "NewEnumerator0")
        (set `self.kickStartTime` (`GameplayStatics.GetTimeSeconds`))
        (set `self.kickStartZ` _returnvalue_z))))
  (:`Canceled`
    (switch `/Game/Footballer/Misc/EKickType` (`self.KickType`) :!label _label_2
      (:`NewEnumerator0`
        _)
      (:`NewEnumerator1`
        _)
      (:`NewEnumerator2`
        _))
    (`self.ResetKick`))
  (:`Completed`
    (goto _label_2)))

(event `OnBallKicked`
  (bind _football (`self.Football`))
  (`self.IncrementStreak`)
  (`/Game/Footballer/Blueprints/BP_Football.SetFireActive` _football (select `int` (`self.StreakStage`) :`0` false :`1` false :`2` true :`3` true))
  (`/Game/Footballer/Blueprints/BP_Football.SetParticleColor` _football (`KismetMathLibrary.LinearColorLerp` (`self.ParticleColor0`) (`self.ParticleColor1`) (`self.PowerRatio`)))
  (if (<= (`KismetMathLibrary.RandomFloat`) (`self.SwitchProbability`))
    (`/Game/Footballer/Blueprints/BP_Football.SwitchSides` _football)))

(fn `CalculateBallSpeed`
  (returns (Speed :type "Float (double-precision)") (PowerRatio :type "Float (double-precision)"))
  (bind _gamemode (`self.GameMode`))
  (bind _returnvalue (`CurveFloat.GetFloatValue` (`self.Curve`) (/ (- (`GameplayStatics.GetTimeSeconds`) (`self.kickStartTime`)) (`self.TotalKickTime`))))
  (set `self.PowerRatio` _returnvalue)
  (return (`KismetMathLibrary.Lerp` (`/Game/Footballer/Gamemode/BP_Gamemode.MinBallAirTime` _gamemode) (`/Game/Footballer/Gamemode/BP_Gamemode.MaxBallAirTime` _gamemode) _returnvalue) _returnvalue))

(fn `DebugDraw`
  (locals (NewLocalVar :type "DataDrivenConsoleVariable Structure"))
  (bind _returnvalue (`KismetSystemLibrary.GetConsoleVariableBoolValue` "footballer.DebugDraw"))
  (if _returnvalue
    (`KismetSystemLibrary.DrawDebugSphere` (`SceneComponent.GetSocketLocation` (`self.Mesh`) "R_Foot") (`self.FootSocketRadius`) 12 (`KismetMathLibrary.Conv_ColorToLinearColor` (`self.DebugColor`)))
    (`KismetSystemLibrary.DrawDebugSphere` (`SceneComponent.GetSocketLocation` (`self.Mesh`) "L_Foot") (`self.FootSocketRadius`) 12 (`KismetMathLibrary.Conv_ColorToLinearColor` (`self.DebugColor`)))))

(fn `IncrementStreak`
  (bind _currentstreak (`self.CurrentStreak`))
  (bind _beststreak (`self.BestStreak`))
  (bind _streakstage (`self.StreakStage`))
  (bind _streakthresholds (`/Game/Footballer/Gamemode/BP_Gamemode.StreakThresholds` (`self.GameMode`)))
  (bind _result (`/Engine/EditorBlueprintResources/StandardMacros.IncrementInt` _currentstreak)
    (:`  `
      (set `self.BestStreak` (`KismetMathLibrary.SelectInt` _currentstreak _beststreak (> _currentstreak _beststreak)))
      (if (and (`KismetArrayLibrary.Array_IsValidIndex` _streakthresholds _streakstage) (>= _result (`|GetArrayItem` _streakthresholds _streakstage)))
        (`/Engine/EditorBlueprintResources/StandardMacros.IncrementInt` (`self.StreakStage`))))))

(fn `InitBall`
  (if (`KismetSystemLibrary.IsValid` (`self.Football`))
    (`/Game/Footballer/Blueprints/BP_Football.EnableSim` (`self.Football`))))

(fn `InitGame`
  (bind (_returnvalue_roll _returnvalue_pitch _returnvalue_yaw) (`KismetMathLibrary.BreakRotator` (`SceneComponent.GetSocketRotation` (`self.Mesh`) "R_Foot")))
  (bind _outactors (`GameplayStatics.GetAllActorsOfClass` "/Game/Footballer/Blueprints/BP_Football.BP_Football_C"))
  (if (`KismetArrayLibrary.Array_IsEmpty` _outactors)
    (`KismetSystemLibrary.PrintString` "Missing Football!!!" true true (struct :`R` 0.270833 :`B` 0.009486 :`A` 1.0))
    (else
      (bind _output_get (set `self.Football` (`|GetArrayItem` _outactors)))
      (`/Game/Footballer/Blueprints/BP_Football.AttachToFootballer` _output_get self)
      (set `self.PrevFootZ` _returnvalue_yaw))))

(fn `IsFootballAboveFoot`
  (params (KickType :type "/Game/Footballer/Misc/EKickType Enum" :default "NewEnumerator0"))
  (returns (ReturnValue :type Boolean))
  (bind (_returnvalue_x _returnvalue_y _returnvalue_z) (`KismetMathLibrary.BreakVector` (`SceneComponent.GetSocketLocation` (`self.Mesh`) (select `/Game/Footballer/Misc/EKickType` KickType :`NewEnumerator0` "L_Foot" :`NewEnumerator1` "R_Foot" :`NewEnumerator2` "R_Foot" :`NewEnumerator3` "R_Foot" :`NewEnumerator4` "R_Foot" :!type "Name"))))
  (bind (_returnvalue_x_2 _returnvalue_y_2 _returnvalue_z_2) (`KismetMathLibrary.BreakVector` (`self.K2_GetActorLocation` (`self.Football`))))
  (return (>= _returnvalue_z_2 _returnvalue_z)))

(fn `IsFootballNearFoot`
  (params (KickType :type "/Game/Footballer/Misc/EKickType Enum" :default "NewEnumerator0"))
  (returns (ReturnValue :type Boolean))
  (return (<= (`KismetMathLibrary.Vector_Distance` (`SceneComponent.GetSocketLocation` (`self.Mesh`) (select `/Game/Footballer/Misc/EKickType` KickType :`NewEnumerator0` "L_Foot" :`NewEnumerator1` "R_Foot" :`NewEnumerator2` "R_Foot" :`NewEnumerator3` "R_Foot" :`NewEnumerator4` "R_Foot" :!type "Name")) (`self.K2_GetActorLocation` (`self.Football`))) (`self.FootSocketRadius`))))

(fn `IsFootMovingUp`
  (params (KickType :type "/Game/Footballer/Misc/EKickType Enum" :default "NewEnumerator0"))
  (returns (isMovingUp :type Boolean))
  (bind (_returnvalue_x _returnvalue_y _returnvalue_z) (`KismetMathLibrary.BreakVector` (`SceneComponent.GetSocketLocation` (`self.Mesh`) (select `/Game/Footballer/Misc/EKickType` KickType :`NewEnumerator0` "L_Foot" :`NewEnumerator1` "R_Foot" :`NewEnumerator2` "R_Foot" :`NewEnumerator3` "R_Foot" :`NewEnumerator4` "R_Foot" :!type "Name"))))
  (return (> _returnvalue_z (`self.PrevFootZ`))))

(fn `LoseStreak`
  (set `self.CurrentStreak` 0)
  (set `self.StreakStage` 0)
  (`/Game/Footballer/Blueprints/BP_Football.SetFireActive` (`self.Football`) false))

(fn `ResetKick`
  (set `self.KickType` "NewEnumerator2")
  (set `self.PrevFootZ` 0.0))

(fn `UpdateFlick`
  (params (KickType :type "/Game/Footballer/Misc/EKickType Enum" :default "NewEnumerator0"))
  (locals (KickTypeLocal :type "/Game/Footballer/Misc/EKickType Enum" :default "NewEnumerator0"))
  (bind (_speed _powerratio) (`self.CalculateBallSpeed`))
  (bind (_returnvalue_x _returnvalue_y _returnvalue_z) (`KismetMathLibrary.BreakVector` (`SceneComponent.GetSocketLocation` (`self.Mesh`) "R_Foot")))
  (set `local.KickTypeLocal` KickType)
  (if (and (`self.IsFootMovingUp` KickType) (`self.IsFootballAboveFoot` KickType))
    ;[1 1 1] foot is moving upwards
    (set `self.DebugColor` (`self.SuccesDebugColor`))
    (if (`self.IsFootballNearFoot` (`local.KickTypeLocal`))
      (bind _successful_kick (`/Game/Footballer/Blueprints/BP_Football.Kicked` (`self.Football`) _speed _powerratio))
      (set `self.KickType` "NewEnumerator2")
      (if _successful_kick
        (`self.OnBallKicked`))
      (else
        (`self.DebugDraw`)
        (set `self.PrevFootZ` _returnvalue_z)))
    (else
      ;[1 1 1] foot is moving downwards
      (set `self.DebugColor` (`self.FailDebugColor`))
      (`self.DebugDraw`)
      (if (`self.IsFootballNearFoot` (`local.KickTypeLocal`))
        (set `self.PowerRatio` 0.0)
        (bind _successful_kick_2 (`/Game/Footballer/Blueprints/BP_Football.Kicked` (`self.Football`) (`/Game/Footballer/Gamemode/BP_Gamemode.MinBallAirTime` (`self.GameMode`)) 0.0))
        (if _successful_kick_2
          (`self.OnBallKicked`))))))

(fn `UserConstructionScript`)